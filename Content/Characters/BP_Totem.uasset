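; Player-controlled totem pawn for Urn Wars that hovers, dashes and aims.
; Tick drives a physics body with trace-fed PID hover, input forces and damping, while dashes add an impulse and a curve-driven spin around an input-derived axis.
; Aiming changes speed, damping, camera distance and FOV, and blocks dashing.
; PlayerState supplies team outline color and a camera-facing nametag, and dissolves play on spawn and death, including attached actors.
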(event Custom|Name%20Updated
  ;[1 1 1] Bind name updated function
  (CallFunction|SetName))

(event Custom|Freeze
  (bind _totemmesh (Variables|Default|GetTotemMesh))
  ;[1 1 1] Freeze and disable collision after dissolved
  (Physics|SetSimulatePhysics _totemmesh false)
  (Collision|SetCollisionEnabled _totemmesh "NoCollision"))

(event Custom|Bind%20Name%20Updated%20Function
  ;[1 1 1] Bind name updated function
  (bind _asbp_totem_player_state (Utilities|Casting|CastToBP_TotemPlayerState (Variables|Default|GetPlayerState)))
  (EventDispatchers|UnbindallEventsfromNameUpdated _asbp_totem_player_state)
  (EventDispatchers|BindEventtoNameUpdated _asbp_totem_player_state (delegate Custom|Name%20Updated)))

(event Custom|SetOutlineVisibility
  (Rendering|SetVisibility (Variables|Default|GetTotemOutline) (not (Pawn|IsLocallyControlled)) true))

(event EventBeginPlay
  (bind _dissolvecomponent (Variables|Default|GetDissolveComponent))
  (Utilities|Time|SetTimerbyEvent (delegate Custom|SetOutlineVisibility) 0.65)
  ;[1 1 1] Call in both places to ensure execution
  (CallFunction|SetAccentColor)
  (CallFunction|SetName)
  (CallFunction|BindNameUpdatedFunction)
  (if true
    (bind _returnvalue (Audio|SpawnSoundAttached "/Game/Audio/SFX/Ambient/AmbientLoopCue.AmbientLoopCue" (Variables|Default|GetTotemMesh) "None" "0, 0, 0" "0, 0, 0" "KeepRelativeOffset" false 1.0 1.0 0.0 0 0))
    (Variables|Default|SetAmbientLoop _returnvalue))
  ;[1 1 1] Dissolve
  (Default|AddAllStaticMeshes _dissolvecomponent)
  (Default|Dissolvein _dissolvecomponent)
  ;[1 1 1] Dissolve in children
  (for _array_element (Actor|GetAttachedActors true)
    (Utilities|IsValid (Actor|GetComponentbyClass _array_element "/Game/Effects/DissolveComponent.DissolveComponent_C")
      (:Is%20Valid
        (Default|Dissolvein (Actor|GetComponentbyClass _array_element "/Game/Effects/DissolveComponent.DissolveComponent_C"))))))

(event EventOnDeath
  (params (KillingDamage :type Float%20%28single-precision%29) (DamageEvent :type Damage%20Event%20Structure%20%28by%20ref%29) (InstigatingPawn :type Pawn%20Object%20Reference) (DamageCauser :type Actor%20Object%20Reference))
  (bind _dissolvecomponent (Variables|Default|GetDissolveComponent))
  (Class|TotemPawn|Disable)
  (Physics|SetEnableGravity (Variables|Default|GetTotemMesh) true)
  (if (Pawn|IsLocallyControlled)
    (Audio|PlaySound2D "/Game/Audio/SFX/Death/YouDiedSoundCue.YouDiedSoundCue" 1.0 1.0 0.0 0 0)
    (else
      (Audio|PlaySoundatLocation "/Game/Audio/SFX/Death/OtherDiedSoundCue.OtherDiedSoundCue" (Transformation|GetActorLocation) "0, 0, 0" 1.0 1.0 0.0 0 0 0)))
  (Default|DissolveOut _dissolvecomponent)
  (EventDispatchers|BindEventtoDissolveFinished _dissolvecomponent (delegate Custom|Freeze))
  (for _array_element (Actor|GetAttachedActors true)
    (Utilities|IsValid (Actor|GetComponentbyClass _array_element "/Game/Effects/DissolveComponent.DissolveComponent_C")
      (:Is%20Valid
        (Default|DissolveOut (Actor|GetComponentbyClass _array_element "/Game/Effects/DissolveComponent.DissolveComponent_C")))
      (:Is%20Not%20Valid
        _))
    (if (Variables|Default|GetShouldUpdateNametag)
      (Rendering|SetVisibility (Variables|Default|GetTotemOutline) false false)
      (bind _returnvalue (Rendering|Material|CreateDynamicMaterialInstance (Variables|Default|GetNametag) 0 0 "None" :!class /Script/Engine.PrimitiveComponent))
      (bind _opacity (Timeline|FadeNametag Play)
        (:Update
          (Rendering|Material|SetScalarParameterValue _returnvalue "Opacity" _opacity :!class /Script/Engine.MaterialInstanceDynamic))))))

(event EventPossessed
  (params (NewController :type Controller%20Object%20Reference))
  (if (not (Networking|IsDedicatedServer))
    ;[1 1 1] Call in both places to ensure execution
    (CallFunction|SetAccentColor)
    (CallFunction|SetName)
    (CallFunction|BindNameUpdatedFunction)))

(event EventTick
  (params (DeltaSeconds :type Float%20%28single-precision%29))
  ;[1 1 1] Tick
  (Utilities|FlowControl|Sequence
    (:then_0
      (if (Variables|Default|GetIsEnabled)
        (|Hover)
        (|TryDash)
        (|Rotation)
        (|UpdateDashFX)
        (|MovementForceandDamping)))
    (:then_1
      (|UpdateCamera)
      (|SoundEffects)
      (|UpdateNametag))))

(event Input|ActionEvents|InputActionDash
  (params (Key :type Key%20Structure :default "None"))
  ;[1 1 1] Input action
  (:Pressed
    (Variables|Default|SetWantsToDash true))
  (:Released
    (Variables|Default|SetWantsToDash false)))

(event Input|ActionEvents|InputActionAim
  (params (Key :type Key%20Structure :default "None"))
  ;[1 1 1] Input action
  (:Pressed
    (Variables|Default|SetAiming true))
  (:Released
    (Variables|Default|SetAiming false)))

(fn ConstructionScript)

(fn CheckInteract)

(fn SetName
  (bind _nametag (Variables|Default|GetNametag))
  (if (Pawn|IsLocallyControlled)
    (Rendering|SetVisibility (Variables|Default|GetNametag) false false)
    (Variables|Default|SetShouldUpdateNametag false)
    (else
      (bind _asbp_totem_player_state (Utilities|Casting|CastToBP_TotemPlayerState (Variables|Default|GetPlayerState)))
      (Rendering|Components|TextRender|SetText _nametag (Utilities|Text|ToText(String) (Variables|/Game/Gameplay/BP_TotemPlayerState.BP_TotemPlayerState_C|GetName _asbp_totem_player_state)))
      (Rendering|Components|TextRender|SetTextRenderColor _nametag (Math|Conversions|ToColor(LinearColor) (Variables|Default|GetAccentColor)))
      (Variables|Default|SetShouldUpdateNametag true))))

(fn SetAccentColor
  (bind _asurn_wars_player_state (Utilities|Casting|CastToUrnWarsPlayerState (Variables|Default|GetPlayerState)))
  (bind _asurn_wars_game_state (Utilities|Casting|CastToUrnWarsGameState (Game|GetGameState)))
  (bind _output_get (Variables|Default|SetAccentColor (Utilities|Array|Get(acopy) (Variables|/Game/Gameplay/UrnWars/UrnWarsGameState.UrnWarsGameState_C|GetTeamAccentColors _asurn_wars_game_state) (Variables|/Game/Gameplay/Team/TeamPlayerState.TeamPlayerState_C|GetTeam _asurn_wars_player_state))))
  (bind _returnvalue (Rendering|Material|CreateDynamicMaterialInstance (Variables|Default|GetTotemOutline) 0 0 "None" :!class /Script/Engine.PrimitiveComponent))
  (Rendering|Material|SetVectorParameterValue _returnvalue "Color" _output_get :!class /Script/Engine.MaterialInstanceDynamic))

(fn OnRepDashEffects
  (if (Variables|Default|GetDashEffects)
    (CallFunction|SpawnDashEffects)))

(fn SpawnDashEffects
  ;[1 1 1] Spawn dash particles
  (bind _returnvalue (Niagara|SpawnSystemAttached "/Game/Effects/Totem/DashTrails.DashTrails" (Variables|Default|GetTotemMesh) "None" "0, 0, 0" "0, 0, 0" "KeepRelativeOffset" true))
  (Variables|Default|SetDashFX _returnvalue))

(event Custom|StopDash
  (Variables|Default|SetIsDashing false))