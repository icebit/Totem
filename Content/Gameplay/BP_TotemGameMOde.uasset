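; Game mode for Totem matches that gates the start on player readiness, relays kills and handles game over.
; Tick polls CheckReady until enough players have joined and all are ready, then runs the game state's countdown component, whose end event calls BeginMatch.
; GameOver notifies every player controller of the winning team and reloads the level after a delay.
; Players spawn at the first SpectatorStart, and OnTotemKilled broadcasts kill details to all controllers.
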(event Custom|BeginMatch
  ;[1 1 1] Begin countdown and start if all ready
  (Variables|Default|SetInProgress true)
  (CallFunction|OnStartMatch))

(event Custom|GameOver
  (params (Winning%20Team :type Integer%20%28by%20ref%29))
  ;[1 1 1] Notify all players on game over
  (if (Variables|Default|GetInProgress)
    (Variables|Default|SetInProgress false)
    (bind _outactors (Actor|GetAllActorsOfClass "/Game/Gameplay/BP_TotemPlayerController.BP_TotemPlayerController_C"))
    (for _array_element _outactors
      (Default|OnGameOver _array_element Winning%20Team))
    ;[1 1 1] Restart game
    (Utilities|Time|SetTimerbyEvent (delegate Custom|Restart%20Level) 8.0)))

(event Custom|Restart%20Level
  ;[1 1 1] Restart game
  (bind _returnvalue (Game|GetCurrentLevelName true))
  (Game|OpenLevel(byName) (Utilities|String|StringToName _returnvalue)))

(event EventTick
  (params (DeltaSeconds :type Float%20%28single-precision%29))
  ;[1 1 1] Try to start match
  (if (not (Variables|Default|GetPendingStart))
    (bind _allready (CallFunction|CheckReady))
    (if _allready
      ;[1 1 1] Begin countdown and start if all ready
      (Variables|Default|SetPendingStart true)
      (bind _asbp_totem_game_state (Utilities|Casting|CastToBP_TotemGameState (Game|GetGameState)))
      (Default|BeginCountdown (Variables|/Game/Gameplay/BP_TotemGameState.BP_TotemGameState_C|GetCountdownComponent _asbp_totem_game_state))
      (EventDispatchers|BindEventtoOnEndCountdown (Variables|/Game/Gameplay/BP_TotemGameState.BP_TotemGameState_C|GetCountdownComponent _asbp_totem_game_state) (delegate Custom|BeginMatch)))))

(fn ConstructionScript)

(fn OnStartMatch)

(fn CheckReady
  ;[1 1 1] If there are enough players...
  (bind _returnvalue (Class|GameModeBase|GetNumPlayers))
  (if (>= _returnvalue (Variables|Default|GetRequiredNumPlayers))
    ;[1 1 1] Check if all are ready. This could be modified to only require a certain percentage to be ready
    (for _array_element (Variables|/Script/Engine.GameStateBase|GetPlayerArray (Game|GetGameState))
      (bind _asbp_totem_player_state (Utilities|Casting|CastToBP_TotemPlayerState _array_element))
      (if (Variables|/Game/Gameplay/BP_TotemPlayerState.BP_TotemPlayerState_C|GetIsReady _asbp_totem_player_state)
        (Math|Integer|IncrementInt (LocalVariables|GetAmountReady))))
    (return (== (LocalVariables|GetAmountReady) _returnvalue))))

(fn FindPlayerStart
  (params (Player :type Controller%20Object%20Reference) (IncomingName :type String))
  (bind _outactors (Actor|GetAllActorsOfClass "/Game/Gameplay/SpectatorStart.SpectatorStart_C"))
  (return (Utilities|Array|Get(acopy) _outactors)))

(fn OnTotemKilled
  (params (Killer :type Controller%20Object%20Reference) (KilledPlayer :type Controller%20Object%20Reference) (KilledPawn :type Pawn%20Object%20Reference) (DamageType :type Damage%20Type%20Object%20Reference))
  (bind _playerstate (Variables|/Script/Engine.Controller|GetPlayerState Killer))
  (Utilities|IsValid Killer
    (:Is%20Valid
      (bind _asbp_totem_player_state (Utilities|Casting|CastToBP_TotemPlayerState _playerstate)
        (:then
          _)
        (:CastFailed
          _))
      (bind _asbp_totem_player_state_2 (Utilities|Casting|CastToBP_TotemPlayerState (Variables|/Script/Engine.Controller|GetPlayerState KilledPlayer)))
      (bind _outactors (Actor|GetAllActorsOfClass "/Game/Gameplay/BP_TotemPlayerController.BP_TotemPlayerController_C"))
      (for _array_element _outactors
        (Default|NotifyTotemKilled _array_element (Variables|/Game/Gameplay/BP_TotemPlayerState.BP_TotemPlayerState_C|GetName _asbp_totem_player_state) (Variables|/Game/Gameplay/BP_TotemPlayerState.BP_TotemPlayerState_C|GetName _asbp_totem_player_state_2) (select (Utilities|IsValid _playerstate) false true) DamageType))
      (return true))))