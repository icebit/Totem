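; Player controller for totem pawns that manages each player's HUD, name and respawn flow.
; It sends the GameInstance name to the server and swaps pre-match, primary HUD, crosshair and respawning widgets on ready, possession and death.
; Death starts a PlayerState countdown that ends in UrnWarsGameMode respawning the player.
; Notify events feed killfeed, out-of-ammo and hit feedback to the widgets; game over hides the crosshair.
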(event Custom|NotifyTotemKilled
  (params (KillerName :type String) (VictimName :type String) (Suicide :type Boolean) (DamageType :type Damage%20Type%20Object%20Reference))
  (bind _primaryhudwidget (Variables|Default|GetPrimaryHUDWidget))
  ;[1 1 1] Update killfeed
  (Utilities|IsValid _primaryhudwidget
    (:Is%20Valid
      (Default|AddtoKillfeed _primaryhudwidget KillerName VictimName Suicide))))

(event Custom|ClientOnGameOver
  (params (Winning%20Team :type Integer))
  ;[1 1 1] Game over
  (CallFunction|SetCrosshairVisibility false)
  (Variables|Default|SetGameOver true))

(event Custom|ServerSetName
  (params (New%20Name :type String))
  (bind _asbp_totem_player_state (Utilities|Casting|CastToBP_TotemPlayerState (Variables|Default|GetPlayerState)))
  (Default|SetName _asbp_totem_player_state New%20Name))

(event Custom|New%20Spectator%20Spawned
  ;[1 1 1] When a new spectator is possessed
)

(event Custom|New%20Totem%20Spawned
  (bind _respawningwidget (Variables|Default|GetRespawningWidget))
  ;[1 1 1] When a new totem is possessed
  ;[1 1 1] Remove pre match widget
  (Widget|RemovefromParent (Variables|Default|GetPreMatchWidget))
  ;[1 1 1] Remove respawning widget if necessary
  (Utilities|IsValid _respawningwidget
    (:Is%20Valid
      (Widget|RemovefromParent _respawningwidget))
    (:Is%20Not%20Valid
      _))
  ;[1 1 1] Remove primary HUD if necessary
  (Utilities|IsValid (Variables|Default|GetPrimaryHUDWidget)
    (:Is%20Valid
      (Widget|RemovefromParent (Variables|Default|GetPrimaryHUDWidget)))
    (:Is%20Not%20Valid
      _))
  ;[1 1 1] Create primary HUD widget
  (bind _returnvalue (UserInterface|CreateWidget "/Game/UI/HUD/PrimaryHUDWidget.PrimaryHUDWidget_C"))
  (Variables|Default|SetPrimaryHUDWidget _returnvalue)
  (Variables|Default|SetPrimaryHUDVisible false)
  (CallFunction|SetPrimaryHUDVisibility true)
  (CallFunction|SetCrosshairVisibility true)
  ;[1 1 1] Fade from black
  (CameraFades|StartCameraFade :self (Game|GetPlayerCameraManager 0) :FromAlpha 1.0 :Duration 1.0))

(event Custom|OnRespawn
  ;[1 1 1] Respawn countdown
  (bind _asbp_totem_player_state (Utilities|Casting|CastToBP_TotemPlayerState (Variables|Default|GetPlayerState)))
  (Default|BeginCountdown (Variables|/Game/Gameplay/BP_TotemPlayerState.BP_TotemPlayerState_C|GetCountdownComponent _asbp_totem_player_state))
  (EventDispatchers|UnbindallEventsfromOnEndCountdown (Variables|/Game/Gameplay/BP_TotemPlayerState.BP_TotemPlayerState_C|GetCountdownComponent _asbp_totem_player_state))
  (EventDispatchers|BindEventtoOnEndCountdown (Variables|/Game/Gameplay/BP_TotemPlayerState.BP_TotemPlayerState_C|GetCountdownComponent _asbp_totem_player_state) (delegate Custom|OnRespawnEndCountdown))
  ;[1 1 1] Inform client of respawn
  (CallFunction|ClientonRespawn))

(event Custom|OnRespawnEndCountdown
  ;[1 1 1] Respawn countdown
  (bind _asurn_wars_game_mode (Utilities|Casting|CastToUrnWarsGameMode (Game|GetGameMode)))
  (Default|DestroyandRespawn _asurn_wars_game_mode self))

(event Custom|OnEndGame)

(event Custom|ClientOnRespawn
  ;[1 1 1] Display respawning widget
  (bind _returnvalue (UserInterface|CreateWidget "/Game/UI/HUD/RespawningWidget.RespawningWidget_C"))
  (bind _output_get (Variables|Default|SetRespawningWidget _returnvalue))
  (UserInterface|Viewport|AddtoViewport _output_get 0)
  (CallFunction|SetCrosshairVisibility false))

(event Custom|OnReady
  ;[1 1 1] Remove ready widget and add pre match widget
  (Variables|Default|SetbShowMouseCursor false)
  (bind _returnvalue (UserInterface|CreateWidget "/Game/UI/HUD/PreMatchWidget.PreMatchWidget_C"))
  (bind _output_get (Variables|Default|SetPreMatchWidget _returnvalue))
  (UserInterface|Viewport|AddtoViewport _output_get 0))

(event Custom|OnGameOver
  (params (Winning%20Team :type Integer))
  ;[1 1 1] Game over
  (Variables|Default|SetGameOver true)
  (CallFunction|ClientonGameOver Winning%20Team))

(event EventPossess
  (params (PossessedPawn :type Pawn%20Object%20Reference))
  ;[1 1 1] Notify client when new totem or spectator is possessed
  (Utilities|Casting|CastToBP_Totem PossessedPawn
    (:then
      (CallFunction|NewTotemSpawned))
    (:CastFailed
      (Utilities|Casting|CastToSpectatorPawn PossessedPawn)
      (CallFunction|NewSpectatorSpawned))))

(event EventNotifyOutOfAmmo
  (bind _primaryhudwidget (Variables|Default|GetPrimaryHUDWidget))
  ;[1 1 1] Out of ammo event
  (Utilities|IsValid _primaryhudwidget
    (:Is%20Valid
      (Default|OutOfAmmo _primaryhudwidget))))

(event EventNotifyHitEnemy
  ;[1 1 1] HUD Notify hit effect
  (Default|NotifyHit (Variables|Default|GetCrosshairWidget)))

(event EventBeginPlay
  (if (Pawn|IsLocalPlayerController)
    (bind _astotem_game_instance (Utilities|Casting|CastToTotemGameInstance (Game|GetGameInstance))
      (:then
        (CallFunction|ServerSetName (Variables|/Game/Gameplay/TotemGameInstance.TotemGameInstance_C|GetName _astotem_game_instance)))
      (:CastFailed
        _))
    ;[1 1 1] Create crosshair
    (bind _returnvalue (UserInterface|CreateWidget "/Game/UI/HUD/CrosshairWidget.CrosshairWidget_C"))
    (Variables|Default|SetCrosshairWidget _returnvalue)
    (CallFunction|SetCrosshairVisibility false)
    ;[1 1 1] Create scoreboard widget
    (bind _returnvalue_2 (UserInterface|CreateWidget (Variables|Default|GetScoreboard%20Class)))
    (Variables|Default|SetScoreboardWidget _returnvalue_2)))

(event EventOnDeath
  (CallFunction|OnRespawn))

(fn ConstructionScript)

(fn SetPrimaryHUDVisibility
  (params (Visible :type Boolean))
  (if Visible
    (if (not (Variables|Default|GetPrimaryHUDVisible))
      (UserInterface|Viewport|AddtoViewport (Variables|Default|GetPrimaryHUDWidget) 0)
      (Variables|Default|SetPrimaryHUDVisible true))
    (elif (Variables|Default|GetPrimaryHUDVisible)
      (Widget|RemovefromParent (Variables|Default|GetPrimaryHUDWidget))
      (Variables|Default|SetPrimaryHUDVisible false))))

(fn SetCrosshairVisibility
  (params (Visible :type Boolean))
  (if Visible
    (if (not (Variables|Default|GetCrosshairVisible))
      (UserInterface|Viewport|AddtoViewport (Variables|Default|GetCrosshairWidget) 0)
      (Variables|Default|SetCrosshairVisible true))
    (elif (Variables|Default|GetCrosshairVisible)
      (Widget|RemovefromParent (Variables|Default|GetCrosshairWidget))
      (Variables|Default|SetCrosshairVisible false))))

(fn SetModeSpecificHUDVisibility
  (params (Visible :type Boolean)))

(fn SetTotemPaused
  (params (Paused :type Boolean))
  (bind _asbp_totem (Utilities|Casting|CastToBP_Totem (Pawn|GetControlledPawn)))
  (Class|TotemPawn|SetPaused _asbp_totem Paused))

(fn OpenPauseMenu)

(fn OpenPrimaryHUD
  (Widget|RemovefromParent (Variables|Default|GetPauseMenu))
  (UserInterface|Viewport|AddtoViewport (Variables|Default|GetCrosshairWidget) 0))